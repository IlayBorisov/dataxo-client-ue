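; Clickable grid tile for a tic-tac-toe style board that displays an X, O or empty state.
; X and O meshes start hidden; a click sends the tile's grid coordinates as a move through BP_WebSocketActor.
; SetSymbol switches mesh visibility, restoring the empty mesh only on reset, and SetTileColor swaps the cube's material between green and red.
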(event EventBeginPlay
  ;[1 1 1] Скрыть символы X и O при запуске
  (Rendering|SetVisibility (Variables|Default|GetXMesh) false false)
  (Rendering|SetVisibility (Variables|Default|GetOMesh) false false))

(event MouseInput|EventActorOnClicked
  (params (ButtonPressed :type Key%20Structure))
  (bind _returnvalue (Actor|GetActorOfClass "/Game/WebSocket/BP_WebSocketActor.BP_WebSocketActor_C"))
  (Class|WebSocketActor|MakeMove _returnvalue (Variables|Default|GetGridX%20) (Variables|Default|GetGridY))
  (Utilities|Casting|CastToMyGameInstance (Game|GetGameInstance)))

(fn ConstructionScript)

(fn SetSymbol
  (params (InputSymbol :type Integer))
  ;[1 1 1] Метод для отображения символа
  (switch int InputSymbol
    (:0
      (Rendering|SetVisibility (Variables|Default|GetOMesh) false false)
      (Rendering|SetVisibility (Variables|Default|GetXMesh) false false)
      (Rendering|SetVisibility (Variables|Default|GetEmptyMesh) true false))
    (:1
      (Rendering|SetVisibility (Variables|Default|GetXMesh) true false))
    (:2
      (Rendering|SetVisibility (Variables|Default|GetOMesh) true false))))

(fn SetTileColor
  (params (ItemColor :type ETileColor%20Enum :default "NewEnumerator0"))
  ;[1 1 1] Метод покраски tile
  (bind _output_get (Variables|Default|SetCurrentTileColor ItemColor))
  (switch Utilities|FlowControl|Switch|SwitchonETileColor _output_get
    (:NewEnumerator0
      (Rendering|Material|SetMaterial (Variables|Default|GetTileCube) 0 "/Game/Materials/M_Tile_Green.M_Tile_Green"))
    (:NewEnumerator1
      (Rendering|Material|SetMaterial (Variables|Default|GetTileCube) 0 "/Game/Materials/M_Tile_Red.M_Tile_Red"))))