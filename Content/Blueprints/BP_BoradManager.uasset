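; BP_BoradManager is a board manager that builds a grid of BP_Tile actors and controls each tile's symbol and color.
; GeneratedGrid spawns tiles spaced by tile size plus padding, stepping along negative X and positive Y, and stores grid coordinates on each.
; Tiles fill a flat row-major array, so PlaceSymbolAt and ChangeColor turn X/Y into an index and forward to that tile.
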(event EventBeginPlay)

(fn ConstructionScript)

(fn GeneratedGrid
  (params (SideX :type Integer) (SideY :type Integer))
  ;[1 1 1] Метод для генерации поля
  (Variables|Default|SetBoardSizeX SideX)
  (Variables|Default|SetBoradSizeY SideY)
  (Variables|Default|SetOffsetX (Math|Float|Truncate (+ (Variables|Default|GetTileSize) (Variables|Default|GetTilePadding))))
  (Variables|Default|SetOffsetY (Math|Float|Truncate (+ (Variables|Default|GetTileSize) (Variables|Default|GetTilePadding))))
  (Variables|Default|SetStartX (Math|Conversions|ToFloat(Integer) (/ (* (* (- (Variables|Default|GetBoardSizeX) 1) (Variables|Default|GetOffsetX)) -1) 2)))
  (Variables|Default|SetStartY (Math|Conversions|ToFloat(Integer) (/ (* (* (- (Variables|Default|GetBoradSizeY) 1) (Variables|Default|GetOffsetY)) -1) 2)))
  (for _index (range 0 (- (Variables|Default|GetBoradSizeY) 1))
    (for _index_2 (range 0 (- (Variables|Default|GetBoardSizeX) 1))
      (bind _output_get (Variables|Default|SetCurrentX (+ (* (* _index_2 (Variables|Default|GetOffsetX)) -1) (Math|Float|Truncate (Variables|Default|GetStartX)))))
      (bind _output_get_2 (Variables|Default|SetCurrentY (+ (* _index (Variables|Default|GetOffsetY)) (Math|Float|Truncate (Variables|Default|GetStartY)))))
      (bind _returnvalue (Game|SpawnActorfromClass "/Game/Blueprints/BP_Tile.BP_Tile_C" (Math|Conversions|ToTransform(Vector) (Math|Vector|MakeVector (Math|Conversions|ToFloat(Integer) _output_get) (Math|Conversions|ToFloat(Integer) _output_get_2) 0.0)) "Undefined" 0 0))
      (Variables|/Game/Blueprints/BP_Tile.BP_Tile_C|SetGridX%20 _returnvalue _index_2)
      (Variables|/Game/Blueprints/BP_Tile.BP_Tile_C|SetGridY _returnvalue _index)
      (bind _output_get_3 (Variables|Default|SetSpawntedTile _returnvalue))
      (Utilities|Array|Add (Variables|Default|GetTilesArray) _output_get_3))))

(fn PlaceSymbolat
  (params (X :type Integer) (Y :type Integer) (Symbol :type Integer))
  ;[1 1 1] Метод для определения поизиции символа
  (bind _output_get (Variables|Default|SetTileIndex (+ (* Y (Variables|Default|GetBoardSizeX)) X)))
  (Default|SetSymbol (Utilities|Array|Get(acopy) (Variables|Default|GetTilesArray) _output_get) Symbol))

(fn ChangeColor
  (params (X :type Integer) (Y :type Integer) (ItemColor :type ETileColor%20Enum :default "NewEnumerator0"))
  ;[1 1 1] Метод для выбора какой tile красить
  (bind _output_get (Variables|Default|SetTileIndex (+ (* Y (Variables|Default|GetBoardSizeX)) X)))
  (Default|SetTileColor (Utilities|Array|Get(acopy) (Variables|Default|GetTilesArray) _output_get) ItemColor))