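; BP_Tile is a clickable grid cell actor for what appears to be a tic-tac-toe style board game.
; It hides its X and O meshes on BeginPlay, and a click asks BP_BoradManager to place symbol 1 at its grid coordinates.
; SetSymbol toggles mesh visibility, fully resetting only for the empty state, while SetTileColor swaps the cube between green and red materials.
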(event EventBeginPlay
  (Rendering|SetVisibility (Variables|Default|GetXMesh) false false)
  (Rendering|SetVisibility (Variables|Default|GetOMesh) false false))

(event MouseInput|EventActorOnClicked
  (params (ButtonPressed :type Key%20Structure :default "None"))
  (bind _returnvalue (Actor|GetActorOfClass "/Game/BP_BoradManager.BP_BoradManager_C"))
  (Default|PlaceSymbolat _returnvalue (Variables|Default|GetGridX%20) (Variables|Default|GetGridY) "NewEnumerator1"))

(fn ConstructionScript)

(fn SetSymbol
  (params (InputSymbol :type EPlayersSymbol%20Enum :default "NewEnumerator0"))
  (bind _output_get (Variables|Default|SetCurrentSymbol InputSymbol))
  (switch Utilities|FlowControl|Switch|SwitchonEPlayersSymbol _output_get
    (:NewEnumerator0
      (Rendering|SetVisibility (Variables|Default|GetOMesh) false false)
      (Rendering|SetVisibility (Variables|Default|GetXMesh) false false)
      (Rendering|SetVisibility (Variables|Default|GetEmptyMesh) true false))
    (:NewEnumerator1
      (Rendering|SetVisibility (Variables|Default|GetXMesh) true false))
    (:NewEnumerator2
      (Rendering|SetVisibility (Variables|Default|GetOMesh) true false))))

(fn SetTileColor
  (params (ItemColor :type ETileColor%20Enum :default "NewEnumerator0"))
  (bind _output_get (Variables|Default|SetCurrentTileColor ItemColor))
  (switch Utilities|FlowControl|Switch|SwitchonETileColor _output_get
    (:NewEnumerator0
      (Rendering|Material|SetMaterial (Variables|Default|GetTileCube) 0 "/Game/M_Tile_Green.M_Tile_Green"))
    (:NewEnumerator1
      (Rendering|Material|SetMaterial (Variables|Default|GetTileCube) 0 "/Game/M_Tile_Red.M_Tile_Red"))))